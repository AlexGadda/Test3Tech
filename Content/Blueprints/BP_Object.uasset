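; BP_Object is a physics sphere with health that hops on a looping timer and can be injured, healed or killed.
; An enum state drives it: Injure starts a per-tick health drain, Heal adds HP and stops the drain, and zero HP means dead.
; Jump impulses derive from target height via √(2gh) and require being alive with jumping enabled.
; Tick also refreshes the health bar widget.
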(event Custom|Jump
  (if (|IsNOTDeadandJumpingisenabled?)
    (Physics|AddImpulse (Variables|Default|GetSphere) (Math|Vector|MakeVector 0.0 0.0 (Variables|transient|GetJumpSpeed)) "None" true)))

(event Custom|Injure
  (if (Utilities|Enum|Equal(Enum) (Variables|State|GetState) "NewEnumerator0")
    (Variables|State|SetState "NewEnumerator1")))

(event Custom|Heal
  (Variables|State|SetCurrentHP (+ (Variables|State|GetCurrentHP) (Variables|State|GetHealAmount)))
  (if (Utilities|Enum|Equal(Enum) (Variables|State|GetState) "NewEnumerator1")
    (Variables|State|SetState "NewEnumerator0")))

(event EventBeginPlay
  ;[0 0 0] Init
  (Variables|State|SetCurrentHP (Variables|Config|GetStartingHP))
  (Variables|transient|SetJumpSpeed (CallFunction|CalcJumpVel (Variables|Config|GetJumpHeight)))
  (Utilities|Time|SetTimerbyEvent (EventDispatchers|CreateEvent :!event Custom|Jump) (Variables|Config|GetJumpInterval) true))

(event EventTick
  (params (DeltaSeconds :type Float%20%28single-precision%29))
  (|UpdateHP)
  (|UpdateWidget))

(fn ConstructionScript)

(fn CalcJumpVel
  (params (Target%20Height :type Float%20%28double-precision%29))
  (return (|(sqrt(((2*g)*y))) 9.8e+02 Target%20Height)))